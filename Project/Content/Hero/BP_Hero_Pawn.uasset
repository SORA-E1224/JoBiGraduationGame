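; Hero pawn Blueprint that handles sword attacks and shield guarding by toggling weapon collision.
; AttackActionEvent triggers the attack on ABP_Hero, while separate start and end events switch Sword and Shield collision, both off at BeginPlay.
; Sword overlaps with actors implementing a required interface pass the damaged actor to ApplyDamage on the GloabalInstance game instance, centralizing damage handling there.
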(event OnComponentBeginOverlap(Sword)
  (params (OverlappedComponent :type Primitive%20Component%20Object%20Reference) (OtherActor :type Actor%20Object%20Reference) (OtherComp :type Primitive%20Component%20Object%20Reference) (OtherBodyIndex :type Integer) (bFromSweep :type Boolean) (SweepResult :type Hit%20Result%20Structure%20%28by%20ref%29))
  ;[1 0 0] Attack
  (if (Utilities|DoesObjectImplementInterface OtherActor "/Script/Graduation_Yoshida.InheritedInterface")
    (bind _asgloabal_instance (Utilities|Casting|CastToGloabalInstance (Game|GetGameInstance)))
    (Class|GloabalInstance|ApplyDamage _asgloabal_instance OtherActor)))

(event Custom|AttackStart
  ;[1 0 0] Attack
  (Collision|SetCollisionEnabled (Variables|Default|GetSword) "QueryOnly"))

(event Custom|AttackEnd
  ;[1 0 0] Attack
  (Collision|SetCollisionEnabled (Variables|Default|GetSword) "NoCollision"))

(event Custom|GuardStart
  ;[0 1 0] Guard
  (Collision|SetCollisionEnabled (Variables|Default|GetShield) "QueryAndPhysics"))

(event Custom|GuardEnd
  ;[0 1 0] Guard
  (Collision|SetCollisionEnabled (Variables|Default|GetShield) "NoCollision"))

(event EventAttackActionEvent
  ;[1 0 0] Attack
  (bind _asabp_hero (Utilities|Casting|CastToABP_Hero (Components|SkeletalMesh|GetAnimInstance (Variables|Character|GetMesh))))
  (Default|Attack _asabp_hero))

(event EventBeginPlay
  ;[1 0 0] Attack
  (CallFunction|AttackEnd)
  ;[0 1 0] Guard
  (CallFunction|GuardEnd))

(fn ConstructionScript)