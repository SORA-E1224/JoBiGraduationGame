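; BP_Goal is a goal actor that sends the game to the Result scene when the player reaches it.
; When the player's pawn overlaps its collision and no fade is running, it starts a white FadeIn on the GloabalInstance's widget.
; The fade's end delegate calls LoadResultScene, which tells the game instance's Manager to set the Result scene.
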(event OnComponentBeginOverlap(CollisionComponent)
  (params (OverlappedComponent :type Primitive%20Component%20Object%20Reference) (OtherActor :type Actor%20Object%20Reference) (OtherComp :type Primitive%20Component%20Object%20Reference) (OtherBodyIndex :type Integer) (bFromSweep :type Boolean) (SweepResult :type Hit%20Result%20Structure%20%28by%20ref%29))
  (bind _asgloabal_instance (Utilities|Casting|CastToGloabalInstance (Game|GetGameInstance)))
  (Utilities|IsValid (Variables|/Script/Graduation_Yoshida.GloabalInstance|Getwidget _asgloabal_instance)
    (:Is%20Valid
      (if (and (Utilities|Enum|Equal(Enum) (Variables|/Script/Graduation_Yoshida.FadeUIWidget|GetCurrentFadeMode (Variables|/Script/Graduation_Yoshida.GloabalInstance|Getwidget _asgloabal_instance)) "FM_None") (== OtherActor (Pawn|GetControlledPawn (Game|GetPlayerController 0))))
        (Class|FadeUIWidget|StartFade (Variables|/Script/Graduation_Yoshida.GloabalInstance|Getwidget _asgloabal_instance) "FM_FadeIn" 1.0 "(R=1.000000,G=1.000000,B=1.000000,A=1.000000)" (Utilities|Struct|MakeFadeEvent (delegate Custom|LoadResultScene)))))))

(event Custom|LoadResultScene
  (Utilities|IsValid (Variables|/Script/Graduation_Yoshida.GloabalInstance|Getmanager (stale OnComponentBeginOverlap(CollisionComponent) _asgloabal_instance))
    (:Is%20Valid
      (Class|SceneManager|SetScene (Variables|/Script/Graduation_Yoshida.GloabalInstance|Getmanager (stale OnComponentBeginOverlap(CollisionComponent) _asgloabal_instance)) "ST_Result"))))

(fn ConstructionScript)