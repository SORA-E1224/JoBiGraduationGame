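; BP_FairyField is a box volume with a grid FieldID that tells BP_FairyManager which fields make up its spawn field list.
; At BeginPlay it caches its own box plus those of orthogonally adjacent fields, found by comparing FieldIDs.
; It pushes that list to the first manager found, both at BeginPlay and whenever something begins overlapping the box.
; The construction script sizes the box from Extent.
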(event OnComponentBeginOverlap(Box)
  (params (OverlappedComponent :type Primitive%20Component%20Object%20Reference) (OtherActor :type Actor%20Object%20Reference) (OtherComp :type Primitive%20Component%20Object%20Reference) (OtherBodyIndex :type Integer) (bFromSweep :type Boolean) (SweepResult :type Hit%20Result%20Structure%20%28by%20ref%29))
  (Utilities|IsValid (Variables|Default|GetFairyManager) :!label _label
    (:Is%20Valid
      (Variables|/Game/Blueprints/Actors/BP_FairyManager.BP_FairyManager_C|SetSpawnFieldList (Variables|Default|GetFairyManager) (Variables|Default|GetNextFieldList)))
    (:Is%20Not%20Valid
      (CallFunction|FindNextField)
      (bind _outactors (Actor|GetAllActorsOfClass "/Game/Blueprints/Actors/BP_FairyManager.BP_FairyManager_C"))
      (Class|ArrayFunctionLibrary|IsEmptyExec _outactors
        (:NotEmpty
          (Variables|Default|SetFairyManager (Utilities|Array|Get(acopy) _outactors))
          (goto _label))))))

(event EventBeginPlay
  (CallFunction|FindNextField :!label _label)
  (bind _outactors (Actor|GetAllActorsOfClass "/Game/Blueprints/Actors/BP_FairyManager.BP_FairyManager_C"))
  (Class|ArrayFunctionLibrary|IsEmptyExec _outactors
    (:NotEmpty
      (Variables|Default|SetFairyManager (Utilities|Array|Get(acopy) _outactors))
      (Utilities|IsValid (Variables|Default|GetFairyManager)
        (:Is%20Valid
          (Variables|/Game/Blueprints/Actors/BP_FairyManager.BP_FairyManager_C|SetSpawnFieldList (Variables|Default|GetFairyManager) (Variables|Default|GetNextFieldList)))
        (:Is%20Not%20Valid
          (goto _label))))))

(fn ConstructionScript
  (Components|Box|SetBoxExtent (Variables|Default|GetBox) (Variables|Shape|GetExtent) true))

(fn FindNextField
  (bind _nextfieldlist (Variables|Default|GetNextFieldList))
  (bind _fieldid (Variables|Default|GetFieldID))
  (Utilities|Array|Clear _nextfieldlist)
  (Utilities|Array|Add _nextfieldlist (Variables|Default|GetBox))
  (bind _outactors (Actor|GetAllActorsOfClass "BP_FairyField_C"))
  (for _array_element _outactors
    (LocalVariables|SetBoxCollisionBuff _array_element)
    (Utilities|FlowControl|Sequence
      (:then_0
        (if (== (.x _fieldid) (.x (Variables|BP_FairyField_C|GetFieldID _array_element)))
          (if (== (Math|Integer|Absolute(Integer) (- (Math|Conversions|ToInteger(Byte) (.y _fieldid)) (Math|Conversions|ToInteger(Byte) (.y (Variables|BP_FairyField_C|GetFieldID _array_element))))) 1)
            (Utilities|Array|Add (Variables|Default|GetNextFieldList) (Variables|BP_FairyField_C|GetBox (LocalVariables|GetBoxCollisionBuff)) :!label _label))))
      (:then_1
        (if (== (.y _fieldid) (.y (Variables|BP_FairyField_C|GetFieldID _array_element)))
          (if (== (Math|Integer|Absolute(Integer) (- (Math|Conversions|ToInteger(Byte) (.x _fieldid)) (Math|Conversions|ToInteger(Byte) (.x (Variables|BP_FairyField_C|GetFieldID _array_element))))) 1)
            (goto _label)))))))