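; Player camera actor that follows the pawn and can lock its view onto a target actor.
; On BeginPlay it moves to the first PlayerStart found and becomes the view target, with following off until SetPlayer enables it.
; While following, Tick sweeps it to the pawn's location and, if TargetActor is valid, smoothly turns it along the pawn-to-target direction with a downward, clamped pitch offset.
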(event EventBeginPlay
  (CallFunction|Initialize))

(event EventTick
  (params (DeltaSeconds :type Float%20%28single-precision%29))
  (bind _returnvalue (Game|Player|GetPlayerPawn 0))
  (bind _targetactor (Variables|Default|GetTargetActor))
  (bind _returnvalue_2 (Transformation|GetActorLocation _returnvalue))
  (bind _returnvalue_3 (Transformation|GetActorLocation _targetactor))
  (bind _returnvalue_4 (Math|Rotator|FindLookatRotation _returnvalue_2 _returnvalue_3))
  (if (Variables|Default|GetIsFollowing)
    (Utilities|IsValid _targetactor
      (:Is%20Valid
        (Transformation|SetActorLocation _returnvalue_2 true false)
        (Transformation|SetActorRotation (Math|Interpolation|RInterpTo (Transformation|GetActorRotation) (Math|Rotator|MakeRotator 0.0 (Math|Float|Clamp(Float) (- (.pitch _returnvalue_4) 3e+01) -5e+01 5e+01) (.yaw _returnvalue_4)) (Utilities|Time|GetWorldDeltaSeconds) 5.0)))
      (:Is%20Not%20Valid
        (Transformation|SetActorLocation _returnvalue_2 true false)))))

(fn ConstructionScript)

(fn SetPlayer
  (Game|Player|SetViewTargetwithBlend (Game|GetPlayerController 0) self 0.0 "VTBlend_Linear" 0.0 false)
  (Transformation|SetActorRotation (Math|Rotator|MakeRotator 0.0 -3e+01 0.0))
  (Variables|Default|SetIsFollowing true))

(fn Initialize
  (bind _outactors (Actor|GetAllActorsOfClass "/Script/Engine.PlayerStart"))
  (if (not (== (Utilities|Array|Length _outactors) 0))
    (Transformation|SetActorLocation (Transformation|GetActorLocation (Utilities|Array|Get(acopy) _outactors)) false false)
    (Transformation|SetActorRotation "-30.000000, 0, 0")
    (Game|Player|SetViewTargetwithBlend (Game|GetPlayerController 0) self 0.0 "VTBlend_Linear" 0.0 false)
    (Variables|Default|SetIsFollowing false)))