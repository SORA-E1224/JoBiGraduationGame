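; Spawn point actor that creates a BP_Fairy_SP at its transform on BeginPlay when AutoSpawn is set.
; Each fairy is initialized with the configured Type and a reference to the spawn point.
; With Loop on, the SpawnFairy dispatcher starts a one-shot SpawnFrequency timer for the next spawn, so respawns are event-driven rather than a looping timer.
; EndPlay clears the dispatcher bindings.
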(event Custom|SpawnFairy
  (bind _returnvalue (Game|SpawnActorfromClass "/Game/Blueprints/Actors/BP_Fairy_SP.BP_Fairy_SP_C" (Transformation|GetActorTransform) "Undefined" 0 0))
  (Default|Initialize _returnvalue (Variables|Default|GetType) self))

(event Custom|CallTimer
  (Utilities|Time|SetTimerbyEvent (delegate Custom|SpawnFairy) (Variables|Default|GetSpawnFrequency)))

(event EventBeginPlay
  (if (Variables|Default|GetAutoSpawn)
    (bind _returnvalue (Game|SpawnActorfromClass "/Game/Blueprints/Actors/BP_Fairy_SP.BP_Fairy_SP_C" (Transformation|GetActorTransform) "Undefined" 0 0))
    (Default|Initialize _returnvalue (Variables|Default|GetType) self)
    (if (Variables|Default|GetLoop)
      (EventDispatchers|BindEventtoSpawnFairyEventDispatcher (delegate Custom|CallTimer)))))

(event EventEndPlay
  (params (EndPlayReason :type EEndPlayReason%20Enum :default "Destroyed"))
  (EventDispatchers|UnbindallEventsfromSpawnFairyEventDispatcher))

(fn ConstructionScript)