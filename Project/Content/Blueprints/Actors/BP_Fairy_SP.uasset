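; BP_Fairy_SP is a special fairy pickup with two types, Collect and High Jump, set along with its spawn point through Initialize.
; Initialize applies the type's material to body and wings, while a timeline rotates the two arms in opposite directions.
; Once initialized, any overlap notifies the spawn point, applies the effect and destroys the actor.
; Collect targets untargeted BP_Fairy actors at the player; High Jump enables high jumping and raises jump velocity.
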(event OnComponentBeginOverlap(Volume)
  (params (OverlappedComponent :type Primitive%20Component%20Object%20Reference) (OtherActor :type Actor%20Object%20Reference) (OtherComp :type Primitive%20Component%20Object%20Reference) (OtherBodyIndex :type Integer) (bFromSweep :type Boolean) (SweepResult :type Hit%20Result%20Structure%20%28by%20ref%29))
  (bind _spawnpoint (Variables|Default|GetSpawnPoint))
  (if (Variables|Default|GetBeInitialized)
    (Utilities|FlowControl|Sequence
      (:then_0
        (Utilities|IsValid _spawnpoint
          (:Is%20Valid
            (Default|CallSpawnFairyEventDispatcher _spawnpoint))))
      (:then_1
        (switch Utilities|FlowControl|Switch|SwitchonE_FairySPType (Variables|Default|GetType)
          (:NewEnumerator0
            (|CollectFairy))
          (:NewEnumerator1
            (|HighJump))))
      (:then_2
        (Actor|DestroyActor)))))

(event EventBeginPlay
  (bind _angle (Timeline|WIngAngle PlayFromStart)
    (:Update
      (Transformation|SetWorldRotation (Variables|Default|GetArmL) (Math|Rotator|MakeRotator (.X (Math|Vector|BreakVector _angle)) (.Y (Math|Vector|BreakVector _angle)) (.Z (Math|Vector|BreakVector _angle))) false false)
      (Transformation|SetWorldRotation (Variables|Default|GetArmR) (Math|Rotator|MakeRotator (.x (* _angle -1.0)) (.y (* _angle -1.0)) (.z (* _angle -1.0))) false false))))

(fn ConstructionScript)

(fn Initialize
  (params (Type :type E_FairySPType%20Enum :default "NewEnumerator0") (SpawnPoint :type BP%20Fairy%20SP%20Spawn%20Point%20Object%20Reference))
  (Variables|Default|SetSpawnPoint SpawnPoint)
  (bind _output_get (Variables|Default|SetType Type))
  (switch Utilities|FlowControl|Switch|SwitchonE_FairySPType _output_get
    (:NewEnumerator0
      (LocalVariables|SetMatBuff "/Game/Graphics/Materials/MI_Fairy_SP_Collect.MI_Fairy_SP_Collect"))
    (:NewEnumerator1
      (LocalVariables|SetMatBuff "/Game/Graphics/Materials/MI_Fairy_SP_HighJump.MI_Fairy_SP_HighJump")))
  (Rendering|Material|SetMaterial (Variables|Default|GetSphere) 0 (LocalVariables|GetMatBuff))
  (Rendering|Material|SetMaterial (Variables|Default|GetWingL) 0 (LocalVariables|GetMatBuff))
  (Rendering|Material|SetMaterial (Variables|Default|GetWingR) 0 (LocalVariables|GetMatBuff))
  (Variables|Default|SetBeInitialized true))