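; Manager actor that keeps spawning Power, Speed and Health fairies in spawn fields, capped per type.
; Tick, throttled by a DoOnce and a spawn-rate delay, compares a random type's count to its maximum before spawning a BP_Fairy within a random field's box.
; SetSpawnList swaps the active fields, destroying fairies overlapping fields left out of the new list.
; Helper functions read, increment and decrement per-type counts.
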(event EventTick
  (params (DeltaSeconds :type Float%20%28single-precision%29))
  (bind _returnvalue (Math|Random|RandomInteger 3))
  (bind _spawnfieldlist (Variables|Default|GetSpawnFieldList))
  (bind _returnvalue_2 (Utilities|Array|Length _spawnfieldlist))
  (bind _returnvalue_3 (Math|Conversions|ToByte(Integer) _returnvalue))
  (bind _returnvalue_4 (Math|Random|RandomInteger _returnvalue_2))
  (bind _returnvalue_5 (Utilities|Enum|ByteToEnumE_FairyType _returnvalue_3))
  (bind _output (Utilities|Array|Get(acopy) _spawnfieldlist _returnvalue_4))
  (bind _box (Variables|/Game/Blueprints/Actors/BP_FairyField.BP_FairyField_C|GetBox _output))
  (Utilities|FlowControl|DoOnce false :!label _label
    (:Completed
      (Utilities|FlowControl|Sequence
        (:then_0
          (Class|ArrayFunctionLibrary|IsEmptyExec _spawnfieldlist
            (:NotEmpty
              (if (not (>= (CallFunction|GetFairyNumbyType (Variables|Default|GetCurrentFairyNum) _returnvalue_5) (CallFunction|GetFairyNumbyType (Variables|Default|GetMaxFairyNum) _returnvalue_5)))
                (bind _returnvalue_6 (Game|SpawnActorfromClass "/Game/Blueprints/Actors/BP_Fairy.BP_Fairy_C" (Math|Transform|MakeTransform (Math|Random|RandomPointinBoundingBox (Transformation|GetWorldLocation _box) (Variables|/Script/Engine.BoxComponent|GetBoxExtent _box)) "0, 0, 0" "1,1,1") "Undefined" 0 0))
                (Utilities|IsValid _returnvalue_6
                  (:Is%20Valid
                    (Default|Initialize _returnvalue_6 _returnvalue_5 self)))))))
        (:then_1
          (Utilities|FlowControl|Delay (Variables|Default|GetFairySpawnRate))
          (goto _label Reset))))))

(fn ConstructionScript)

(fn GetAllFairyNum
  (params (value :type S%20Fairy%20Num%20Structure))
  (return (+ (.power value) (.speed value) (.health value))))

(fn SetSpawnList
  (params (list :type Array%20of%20BP%20Fairy%20Field%20Object%20References))
  (bind _destroylist (LocalVariables|GetDestroyList))
  (Utilities|Array|Clear (LocalVariables|GetDestroyList))
  (Utilities|FlowControl|Sequence
    (:then_0
      (Class|ArrayFunctionLibrary|IsEmptyExec (Variables|Default|GetSpawnFieldList)
        (:NotEmpty
          (for _array_element (Variables|Default|GetSpawnFieldList)
            (if (not (Utilities|Array|ContainsItem list _array_element))
              (for _array_element_2 (Collision|GetOverlappingActors (Variables|/Game/Blueprints/Actors/BP_FairyField.BP_FairyField_C|GetBox _array_element) "/Game/Blueprints/Actors/BP_Fairy.BP_Fairy_C" :!class /Script/Engine.PrimitiveComponent)
                (Utilities|IsValid _array_element_2
                  (:Is%20Valid
                    (bind _asbp_fairy (Utilities|Casting|CastToBP_Fairy _array_element_2))
                    (Utilities|Array|Add (LocalVariables|GetDestroyList) _asbp_fairy)))))))))
    (:then_1
      (Variables|Default|SetSpawnFieldList list)
      (Class|ArrayFunctionLibrary|IsEmptyExec _destroylist
        (:NotEmpty
          (for _array_element_3 _destroylist
            (Default|Destroy _array_element_3)))))))

(fn GetFairyNumbyType
  (params (FairyNum :type S%20Fairy%20Num%20Structure) (type :type E_FairyType%20Enum :default "NewEnumerator0"))
  (switch Utilities|FlowControl|Switch|SwitchonE_FairyType type
    (:NewEnumerator0
      (return (.power FairyNum)))
    (:NewEnumerator1
      (return (.speed FairyNum)))
    (:NewEnumerator2
      (return (.health FairyNum)))))

(fn IncrementFairyNumbyType
  (params (fairyNum :type S%20Fairy%20Num%20Structure%20%28by%20ref%29) (type :type E_FairyType%20Enum :default "NewEnumerator0"))
  (bind (_power _speed _health) (Utilities|Struct|BreakS_FairyNum fairyNum))
  (switch Utilities|FlowControl|Switch|SwitchonE_FairyType type
    (:NewEnumerator0
      (Math|Integer|IncrementInt _power))
    (:NewEnumerator1
      (Math|Integer|IncrementInt _speed))
    (:NewEnumerator2
      (Math|Integer|IncrementInt _health))))

(fn DecrementFairyNumbyType
  (params (fairyNum :type S%20Fairy%20Num%20Structure%20%28by%20ref%29) (type :type E_FairyType%20Enum :default "NewEnumerator0"))
  (bind (_power _speed _health) (Utilities|Struct|BreakS_FairyNum fairyNum))
  (switch Utilities|FlowControl|Switch|SwitchonE_FairyType type
    (:NewEnumerator0
      (Math|Integer|DecrementInt _power))
    (:NewEnumerator1
      (Math|Integer|DecrementInt _speed))
    (:NewEnumerator2
      (Math|Integer|DecrementInt _health))))