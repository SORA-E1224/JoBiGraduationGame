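; BP_Fairy is a fairy actor that comes in Power, Speed or Health types and reports itself to a fairy manager.
; Initialize stores the type and manager, sets the sphere material for that type, and increments the manager's count for it.
; Destroy decrements that count and destroys the actor, first looking up a BP_FairyManager in the level if the stored reference is invalid.
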(fn ConstructionScript)

(fn Initialize
  (params (FairyType :type E_FairyType%20Enum :default "NewEnumerator0") (fairyManager :type BP%20Fairy%20Manager%20Object%20Reference))
  (Variables|Default|SetFairyManager fairyManager)
  (bind _output_get (Variables|Default|SetFairyType FairyType))
  (switch Utilities|FlowControl|Switch|SwitchonE_FairyType _output_get
    (:NewEnumerator0
      (LocalVariables|SetmatBuff "/Game/Graphics/Materials/MI_Fairy_Power.MI_Fairy_Power"))
    (:NewEnumerator1
      (LocalVariables|SetmatBuff "/Game/Graphics/Materials/M_Fairy_Speed.M_Fairy_Speed"))
    (:NewEnumerator2
      (LocalVariables|SetmatBuff "/Game/Graphics/Materials/M_Fairy_Health.M_Fairy_Health")))
  (Rendering|Material|SetMaterial (Variables|Default|GetSphere) 0 (LocalVariables|GetmatBuff))
  (Default|IncrementFairyNumbyType (Variables|Default|GetFairyManager) (Variables|/Game/Blueprints/Actors/BP_FairyManager.BP_FairyManager_C|GetCurrentFairyNum (Variables|Default|GetFairyManager)) (Variables|Default|GetFairyType)))

(fn Destroy
  (Utilities|IsValid (Variables|Default|GetFairyManager) :!label _label
    (:Is%20Valid
      (Default|DecrementFairyNumbyType (Variables|Default|GetFairyManager) (Variables|/Game/Blueprints/Actors/BP_FairyManager.BP_FairyManager_C|GetCurrentFairyNum (Variables|Default|GetFairyManager)) (Variables|Default|GetFairyType))
      (Actor|DestroyActor))
    (:Is%20Not%20Valid
      (bind _outactors (Actor|GetAllActorsOfClass "/Game/Blueprints/Actors/BP_FairyManager.BP_FairyManager_C"))
      (Class|ArrayFunctionLibrary|IsEmptyExec _outactors
        (:NotEmpty
          (Variables|Default|SetFairyManager (Utilities|Array|Get(acopy) _outactors))
          (goto _label))))))