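; BP_Scarecrows is a scarecrow actor that reacts to hits by displaying the damage value, with no health tracking.
; Its Damage event spawns a BP_DamageWidget targeted above the actor, passes it the value and plays its fade animation.
; Each accepted hit starts a brief invincibility window, counted down on Tick, during which further Damage events are ignored.
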(event EventTick
  (params (DeltaSeconds :type Float%20%28single-precision%29))
  (if (Variables|Default|GetIsInvincible)
    (bind _output_get (Variables|Default|SetCoolTimer (- (Variables|Default|GetCoolTimer) DeltaSeconds)))
    (if (<= _output_get 0.0)
      (Variables|Default|SetCoolTimer 0.0)
      (Variables|Default|SetIsInvincible false))))

(event EventDamage
  (params (Damage :type Integer) (DamageType :type Damage%20Type%20Object%20Reference) (InstigatedBy :type Controller%20Object%20Reference) (DamageCauser :type Actor%20Object%20Reference))
  (if (not (Variables|Default|GetIsInvincible))
    (bind _returnvalue (UserInterface|CreateWidget "/Game/Blueprints/Widgets/BP_DamageWidget.BP_DamageWidget_C"))
    (Variables|/Game/Blueprints/Widgets/BP_DamageWidget.BP_DamageWidget_C|SetTargetLocation _returnvalue (+ (Transformation|GetActorLocation) "0, 0,100.000000"))
    (Variables|/Game/Blueprints/Widgets/BP_DamageWidget.BP_DamageWidget_C|SetValue _returnvalue Damage)
    (UserInterface|Viewport|AddtoViewport _returnvalue 0)
    (UserInterface|Animation|PlayAnimation _returnvalue (Variables|/Game/Blueprints/Widgets/BP_DamageWidget.BP_DamageWidget_C|GetDamageFade _returnvalue) 0.0 1 "Forward" 1.0)
    (Variables|Default|SetIsInvincible true)
    (Variables|Default|SetCoolTimer 0.1)))

(fn ConstructionScript)