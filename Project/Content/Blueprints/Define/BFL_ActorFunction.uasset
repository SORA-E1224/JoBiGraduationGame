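; Blueprint function library of actor helpers, currently providing a single SetActive function.
; SetActive toggles an actor on or off as a whole by setting its hidden-in-game state, collision and tick together from one boolean.
; An IsValid check guards the call, so invalid actors are ignored.
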(fn SetActive
  (params (Actor :type Actor%20Object%20Reference) (Active :type Boolean))
  (Utilities|IsValid Actor
    (:Is%20Valid
      (Rendering|SetActorHiddenInGame Actor (not Active))
      (Collision|SetActorEnableCollision Actor Active)
      (Actor|Tick|SetActorTickEnabled Actor Active))))