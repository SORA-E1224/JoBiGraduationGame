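; BP_Fairy is a Power, Speed or Health fairy that bobs in place until an actor overlaps its volume, then homes in on it.
; Initialize sets the sphere's material by type, registers with BP_FairyManager's per-type count and stores the hover origin.
; Homing applies a steadily growing force toward the target while clamping physics velocity to constant speed, tightening the turn.
; Destroy decrements the manager's count, looking the manager up if missing.
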(event OnComponentBeginOverlap(Volume)
  (params (OverlappedComponent :type Primitive%20Component%20Object%20Reference) (OtherActor :type Actor%20Object%20Reference) (OtherComp :type Primitive%20Component%20Object%20Reference) (OtherBodyIndex :type Integer) (bFromSweep :type Boolean) (SweepResult :type Hit%20Result%20Structure%20%28by%20ref%29))
  (Utilities|IsValid (Variables|Default|GetTarget)
    (:Is%20Not%20Valid
      (Variables|Default|SetTarget OtherActor)
      (Variables|Default|SetTimer 0.0))))

(event EventTick
  (params (DeltaSeconds :type Float%20%28single-precision%29))
  (Utilities|IsValid (Variables|Default|GetTarget)
    (:Is%20Valid
      (CallFunction|FollowPlayer 2e+03 1e+04))
    (:Is%20Not%20Valid
      (bind _returnvalue (Class|MyMathFunctionLibrary|AddAssignFloat (Variables|Default|GetTimer) (* (Utilities|Time|GetWorldDeltaSeconds) 1.5)))
      (Transformation|SetActorLocation (+ (Variables|Default|GetDefaultLocation) (Math|Vector|MakeVector 0.0 0.0 (* (Math|Trig|Sin(Radians) _returnvalue) 3e+01))) false false))))

(fn ConstructionScript)

(fn Initialize
  (params (FairyType :type E_FairyType%20Enum :default "NewEnumerator0") (fairyManager :type BP%20Fairy%20Manager%20Object%20Reference))
  (Variables|Default|SetFairyManager fairyManager)
  (bind _output_get (Variables|Default|SetFairyType FairyType))
  (switch Utilities|FlowControl|Switch|SwitchonE_FairyType _output_get
    (:NewEnumerator0
      (LocalVariables|SetmatBuff "/Game/Graphics/Materials/MI_Fairy_Power.MI_Fairy_Power"))
    (:NewEnumerator1
      (LocalVariables|SetmatBuff "/Game/Graphics/Materials/MI_Fairy_Speed.MI_Fairy_Speed"))
    (:NewEnumerator2
      (LocalVariables|SetmatBuff "/Game/Graphics/Materials/MI_Fairy_Health.MI_Fairy_Health")))
  (Rendering|Material|SetMaterial (Variables|Default|GetSphere) 0 (LocalVariables|GetmatBuff))
  (Default|IncrementFairyNumbyType (Variables|Default|GetFairyManager) (Variables|/Game/Blueprints/Actors/BP_FairyManager.BP_FairyManager_C|GetCurrentFairyNum (Variables|Default|GetFairyManager)) (Variables|Default|GetFairyType))
  (Variables|Default|SetTimer 0.0)
  (Variables|Default|SetDefaultLocation (Transformation|GetActorLocation)))

(fn Destroy
  (Utilities|IsValid (Variables|Default|GetFairyManager) :!label _label
    (:Is%20Valid
      (Default|DecrementFairyNumbyType (Variables|Default|GetFairyManager) (Variables|/Game/Blueprints/Actors/BP_FairyManager.BP_FairyManager_C|GetCurrentFairyNum (Variables|Default|GetFairyManager)) (Variables|Default|GetFairyType))
      (Actor|DestroyActor))
    (:Is%20Not%20Valid
      (bind _outactors (Actor|GetAllActorsOfClass "/Game/Blueprints/Actors/BP_FairyManager.BP_FairyManager_C"))
      (Class|ArrayFunctionLibrary|IsEmptyExec _outactors
        (:NotEmpty
          (Variables|Default|SetFairyManager (Utilities|Array|Get(acopy) _outactors))
          (goto _label))))))

(fn FollowPlayer
  (params (AdjustSpeed :type Float%20%28single-precision%29) (TimerRate :type Float%20%28single-precision%29))
  (Class|MyMathFunctionLibrary|AddAssignFloat (Variables|Default|GetTimer) (* (Utilities|Time|GetWorldDeltaSeconds) TimerRate))
  (Physics|AddForce (Variables|Default|GetSphere) (* (Math|Vector|Normalize (- (Transformation|GetActorLocation (Variables|Default|GetTarget)) (Transformation|GetActorLocation))) (Variables|Default|GetTimer)) "None" true)
  (Physics|SetPhysicsLinearVelocity (Variables|Default|GetSphere) (* (Math|Vector|Normalize (Transformation|GetVelocity)) AdjustSpeed) false "None"))