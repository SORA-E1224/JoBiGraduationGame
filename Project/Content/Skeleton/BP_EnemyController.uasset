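; AI controller for skeleton enemies that drives BT_Enemy through BB_Enemy and handles life, damage popups and death.
; On BeginPlay it possesses an uncontrolled skeleton if needed and spawns a movable-area volume as a leash.
; Perception inside that area sets the target and run speed; stimulus expiry or leaving the area restores waiting and walk speed.
; Animation dispatchers toggle the attack flag, and Tick calls RunBehaviorTree every frame.
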(event OnPerceptionUpdated(AIPerception)
  (params (UpdatedActors :type Array%20of%20Actor%20Object%20References))
  (|FindingTarget UpdatedActors))

(event Custom|AnyDamage
  (params (Damage :type Integer) (DamageType :type Damage%20Type%20Object%20Reference) (InstigatedBy :type Controller%20Object%20Reference) (DamageCauser :type Actor%20Object%20Reference))
  (Utilities|FlowControl|Sequence
    (:then_0
      (|BeingDamaged Damage))
    (:then_1
      (|DamageView Damage))))

(event EventBeginPlay
  (|InitializeValue)
  (bind _returnvalue (|SetEnemyMovableArea))
  (|SetEnemyAI _returnvalue)
  (|BindEvent))

(event EventTick
  (params (DeltaSeconds :type Float%20%28single-precision%29))
  (AI|RunBehaviorTree "/Game/AI/BT_Enemy.BT_Enemy")
  (|MissingTarget))

(fn ConstructionScript)

(event Custom|OutColisionEvent
  (params (OverlappedComponent :type Primitive%20Component%20Object%20Reference) (OtherActor :type Actor%20Object%20Reference) (OtherComp :type Primitive%20Component%20Object%20Reference) (OtherBodyIndex :type Integer))
  (bind _enemybb (Variables|Default|GetEnemyBB))
  (if (== OtherActor (Pawn|GetControlledPawn))
    (Variables|Default|SetSightTarget 0)
    (AI|Components|Blackboard|SetValueasObject _enemybb (Utilities|Name|MakeLiteralName "PlayerActor") 0)
    (AI|Components|Blackboard|SetValueasBool _enemybb (Utilities|Name|MakeLiteralName "IsWait") true)
    (bind _asbp_enemy_skeleton (Utilities|Casting|CastToBP_Enemy_Skeleton (Pawn|GetControlledPawn)))
    (Variables|/Script/Engine.CharacterMovementComponent|SetMaxWalkSpeed (Variables|/Script/Engine.Character|GetCharacterMovement _asbp_enemy_skeleton) (Variables|/Game/Skeleton/BP_Enemy_Skeleton.BP_Enemy_Skeleton_C|GetWalkSpeed _asbp_enemy_skeleton))))

(event Custom|AttackBegin
  (AI|Components|Blackboard|SetValueasBool (Variables|Default|GetEnemyBB) (Utilities|Name|MakeLiteralName "IsAttack") true))

(event Custom|AttackEnd
  (AI|Components|Blackboard|SetValueasBool (Variables|Default|GetEnemyBB) (Utilities|Name|MakeLiteralName "IsAttack") false))