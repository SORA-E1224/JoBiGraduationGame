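; Skeleton enemy character that forwards received damage to BP_EnemyController and relays damage, attack and death animations to ABP_Enemy_Skeleton.
; Death flags the anim instance as dead and makes the capsule ignore pawns and several custom trace channels.
; Weapon collision is disabled on BeginPlay, and its overlap event applies fixed damage to the overlapped actor.
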(event OnComponentBeginOverlap(WeaponCollision)
  (params (OverlappedComponent :type Primitive%20Component%20Object%20Reference) (OtherActor :type Actor%20Object%20Reference) (OtherComp :type Primitive%20Component%20Object%20Reference) (OtherBodyIndex :type Integer) (bFromSweep :type Boolean) (SweepResult :type Hit%20Result%20Structure%20%28by%20ref%29))
  (Class|BattleFunctionLibrary|ApplyDamage OtherActor 1))

(event Custom|DamageAnim
  (bind _asabp_enemy_skeleton (Utilities|Casting|CastToABP_Enemy_Skeleton (Components|SkeletalMesh|GetAnimInstance (Variables|Character|GetMesh))))
  (Default|DamageAnim _asabp_enemy_skeleton))

(event Custom|DeathAnim
  (bind _capsulecomponent (Variables|Default|GetCapsuleComponent))
  (bind _asabp_enemy_skeleton (Utilities|Casting|CastToABP_Enemy_Skeleton (Components|SkeletalMesh|GetAnimInstance (Variables|Character|GetMesh))))
  (Variables|/Game/Skeleton/ABP_Enemy_Skeleton.ABP_Enemy_Skeleton_C|SetIsDead _asabp_enemy_skeleton true)
  (Collision|SetCollisionResponsetoChannel _capsulecomponent "ECC_Pawn" "ECR_Ignore")
  (Collision|SetCollisionResponsetoChannel _capsulecomponent "ECC_GameTraceChannel3" "ECR_Ignore")
  (Collision|SetCollisionResponsetoChannel _capsulecomponent "ECC_GameTraceChannel4" "ECR_Ignore")
  (Collision|SetCollisionResponsetoChannel _capsulecomponent "ECC_GameTraceChannel5" "ECR_Ignore"))

(event Custom|AttackAnim
  (bind _asabp_enemy_skeleton (Utilities|Casting|CastToABP_Enemy_Skeleton (Components|SkeletalMesh|GetAnimInstance (Variables|Character|GetMesh))))
  (Default|Attack _asabp_enemy_skeleton))

(event EventDamage
  (params (Damage :type Integer) (DamageType :type Damage%20Type%20Object%20Reference) (InstigatedBy :type Controller%20Object%20Reference) (DamageCauser :type Actor%20Object%20Reference))
  (bind _asbp_enemy_controller (Utilities|Casting|CastToBP_EnemyController (Pawn|GetController)))
  (Default|AnyDamage _asbp_enemy_controller Damage DamageType InstigatedBy DamageCauser))

(event EventBeginPlay
  (Collision|SetCollisionEnabled (Variables|Default|GetWeaponCollision) "NoCollision"))

(fn ConstructionScript)